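; Oxygen pickup for a VR game that refills the player's oxygen, which is stored on VRGameMode.
; Its Pickup event adds a fixed amount only when oxygen is below the maximum, then clamps it to that cap.
; A successful pickup plays a 2D sound, writes a non-alert message through WriteToArm and destroys the actor.
; At full oxygen the event does nothing, leaving the item in place.
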(event EventBeginPlay)

(event EventTick
  (params (DeltaSeconds :type Float%20%28single-precision%29)))

(event EventPickup
  (params (AttachTo :type Scene%20Component%20Object%20Reference))
  (bind _asvrgame_mode (Utilities|Casting|CastToVRGameMode (Game|GetGameMode)))
  (if (< (Variables|/Game/Blueprints/VRGameMode.VRGameMode_C|GetPlayerOxygen _asvrgame_mode) 100)
    (Variables|/Game/Blueprints/VRGameMode.VRGameMode_C|SetPlayerOxygen _asvrgame_mode (+ (Variables|/Game/Blueprints/VRGameMode.VRGameMode_C|GetPlayerOxygen _asvrgame_mode) 20))
    (Utilities|FlowControl|Sequence
      (:then_0
        (if (> (Variables|/Game/Blueprints/VRGameMode.VRGameMode_C|GetPlayerOxygen _asvrgame_mode) 100)
          (Variables|/Game/Blueprints/VRGameMode.VRGameMode_C|SetPlayerOxygen _asvrgame_mode 100)))
      (:then_1
        (Audio|PlaySound2D "/Game/Audio/SFX/ItemPickup.ItemPickup" 0.5)
        (bind _asvrgame_mode_2 (Utilities|Casting|CastToVRGameMode (Game|GetGameMode)))
        (Default|WritetoArm _asvrgame_mode_2 "Picked up oxygen" false))
      (:then_2
        (Actor|DestroyActor)))))

(fn ConstructionScript)