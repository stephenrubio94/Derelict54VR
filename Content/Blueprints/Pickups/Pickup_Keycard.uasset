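; Keycard pickup that grants the player a key and then removes itself from the world.
; On pickup it sets the key at its ItemID index to true in DerelictGameMode's Keys array.
; It then has the game mode write a non-alert pickup message with the keycard's name to the arm, plays a pickup sound and destroys the actor.
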(event EventPickup
  (params (AttachTo :type Scene%20Component%20Object%20Reference))
  (bind _asderelict_game_mode (Utilities|Casting|CastToDerelictGameMode (Game|GetGameMode)))
  (Utilities|Array|SetArrayElem (Variables|/Game/Blueprints/DerelictGameMode.DerelictGameMode_C|GetKeys _asderelict_game_mode) (Variables|Default|GetItemID) true)
  (bind _asderelict_game_mode_2 (Utilities|Casting|CastToDerelictGameMode (Game|GetGameMode)))
  (Default|WritetoArm _asderelict_game_mode_2 (Utilities|String|Append (Utilities|String|ToString(Name) (Variables|Default|GetKeycardName)) " picked up") false)
  (Audio|PlaySound2D "/Game/Audio/SFX/ItemPickup.ItemPickup" 0.5)
  (Actor|DestroyActor))

(fn ConstructionScript)