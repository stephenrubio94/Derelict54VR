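; Interactable VR door that slides open when triggered through Pickup, if its key and power requirements are met.
; IsUnlocked checks the game mode's key and power arrays, writing failures to the player's arm display, and failed attempts play a locked sound.
; A timeline lerps the door open with sound, then reverses after a delay.
; The door with a special ID instead ends the game with an airlock sound.
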(event OnComponentBeginOverlap(Box)
  (params (OverlappedComponent :type Primitive%20Component%20Object%20Reference) (OtherActor :type Actor%20Object%20Reference) (OtherComp :type Primitive%20Component%20Object%20Reference) (OtherBodyIndex :type Integer) (bFromSweep :type Boolean) (SweepResult :type Hit%20Result%20Structure%20%28by%20ref%29)))

(event OnComponentEndOverlap(Box)
  (params (OverlappedComponent :type Primitive%20Component%20Object%20Reference) (OtherActor :type Actor%20Object%20Reference) (OtherComp :type Primitive%20Component%20Object%20Reference) (OtherBodyIndex :type Integer)))

(event EventPickup
  (params (AttachTo :type Scene%20Component%20Object%20Reference))
  (Utilities|IsUnlocked
    (:True
      (if (== (Variables|Default|GetDoorID) 9)
        (bind _asvrgame_mode (Utilities|Casting|CastToVRGameMode (Game|GetGameMode)))
        (Default|EndGame _asvrgame_mode)
        (Audio|PlaySoundatLocation "/Game/Audio/SFX/airlockclose.airlockclose" (Transformation|GetActorLocation))
        (else
          (Audio|Components|Audio|Play (Variables|Default|GetDoorOpenSound) 0.0)
          (Utilities|FlowControl|Sequence
            (:then_0
              (bind _doorposition (Timeline|DoorOpenTimeline Play)
                (:Update
                  (Transformation|SetRelativeLocation (Variables|Default|GetDoor) (Math|Vector|Lerp(Vector) (Variables|Default|GetDoorClosed) (Variables|Default|GetDoorOpen) _doorposition) false false))))
            (:then_1
              (Utilities|FlowControl|Delay 5.0)
              (Audio|Components|Audio|Play (Variables|Default|GetDoorOpenSound) 0.0)
              (Timeline|DoorOpenTimeline Reverse))))))
    (:False
      (Audio|PlaySoundatLocation "/Game/Audio/SFX/DoorLocked.DoorLocked" (Transformation|GetWorldLocation (Variables|Default|GetDefaultSceneRoot))))))

(fn ConstructionScript
  (|CallParentFunction))