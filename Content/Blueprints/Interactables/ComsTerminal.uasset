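; Interactable comms terminal that responds to pickup based on the main power state held in DerelictGameMode.
; With power on, it fires only once: it powers a door entry in the game mode's DoorPower array, plays a connection sound, then after a short delay a typing sound and a dialog.
; With power off, it plays the connection sound and writes a main-power error to the arm display on every attempt.
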(event EventPickup
  (params (AttachTo :type Scene%20Component%20Object%20Reference))
  (bind _asderelict_game_mode (Utilities|Casting|CastToDerelictGameMode (Game|GetGameMode)))
  (if (Variables|/Game/Blueprints/DerelictGameMode.DerelictGameMode_C|GetIsMainPowerOn _asderelict_game_mode)
    (if (not (Variables|Default|GetDisplayingMessage_0))
      (Variables|Default|SetDisplayingMessage_0 true)
      (Utilities|Array|SetArrayElem (Variables|/Game/Blueprints/DerelictGameMode.DerelictGameMode_C|GetDoorPower _asderelict_game_mode) 9 true)
      (Audio|PlaySound2D "/Game/Audio/SFX/AlienConnection.AlienConnection")
      (Utilities|FlowControl|Delay 2.0)
      (Audio|PlaySound2D "/Game/Audio/SFX/type.type")
      (bind _asderelict_game_mode_2 (Utilities|Casting|CastToDerelictGameMode (Game|GetGameMode)))
      (Default|PlayDialog _asderelict_game_mode_2 1))
    (else
      (Audio|PlaySound2D "/Game/Audio/SFX/AlienConnection.AlienConnection")
      (bind _asderelict_game_mode_3 (Utilities|Casting|CastToDerelictGameMode (Game|GetGameMode)))
      (Default|WritetoArm _asderelict_game_mode_3 "ERROR: Main Power Disabled" false))))

(fn ConstructionScript
  (|CallParentFunction))