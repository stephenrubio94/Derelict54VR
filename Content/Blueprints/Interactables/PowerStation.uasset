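; Interactable power terminal that the player repairs with a repair kit to raise system power.
; Pickup spends a GameMode kit, increments TotalPower, hides sparks, plays a sound and writes to the arm display, or reports a missing kit.
; The first terminal also powers a door, stops the klaxon, turns on linked lights and plays delayed dialog.
; Other terminals trigger dialog when total power reaches six.
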(event EventPickup
  (params (AttachTo :type Scene%20Component%20Object%20Reference))
  (bind _asgame_mode (Utilities|Casting|CastToGameMode (Game|GetGameMode)))
  (if (Variables|Default|GetIsBroken)
    (if (> (Variables|/Game/Blueprints/GameMode.GameMode_C|GetNumRepairKits _asgame_mode) 0)
      (if (Variables|Default|GetIsFirstTerminal)
        (Utilities|Array|SetArrayElem (Variables|/Game/Blueprints/GameMode.GameMode_C|GetDoorPower _asgame_mode) 7 true))
      (Variables|/Game/Blueprints/GameMode.GameMode_C|SetTotalPower _asgame_mode (+ (Variables|/Game/Blueprints/GameMode.GameMode_C|GetTotalPower _asgame_mode) 1))
      (Audio|PlaySoundatLocation "/Game/Audio/SFX/poweron.poweron" (Transformation|GetActorLocation self))
      (Variables|/Game/Blueprints/GameMode.GameMode_C|SetNumRepairKits _asgame_mode (- (Variables|/Game/Blueprints/GameMode.GameMode_C|GetNumRepairKits _asgame_mode) 1))
      (Variables|Default|SetIsBroken false)
      (Rendering|ToggleVisibility (Variables|Default|GetSparks) false)
      (bind _asgame_mode_2 (Utilities|Casting|CastToGameMode (Game|GetGameMode)))
      (Default|WritetoArm _asgame_mode_2 "Terminal repaired, system power increased" false)
      (if (Variables|Default|GetIsFirstTerminal)
        (Audio|Components|Audio|Stop (Variables|/Script/Engine.AmbientSound|GetAudioComponent (Variables|Default|GetKlaxon)))
        (for _array_element (Variables|Default|GetToggledLights)
          (Rendering|ToggleVisibility (Variables|/Script/Engine.Light|GetLightComponent _array_element) true))
        (Utilities|FlowControl|Delay 5.0)
        (bind _asgame_mode_3 (Utilities|Casting|CastToGameMode (Game|GetGameMode)))
        (Utilities|Array|SetArrayElem (Variables|/Game/Blueprints/GameMode.GameMode_C|GetDoorPower _asgame_mode_3) 7 true)
        (Default|PlayDialog _asgame_mode_3)
        (elif (== (Variables|/Game/Blueprints/GameMode.GameMode_C|GetTotalPower _asgame_mode_2) 6)
          (Default|PlayDialog _asgame_mode_2)))
      (else
        (Audio|PlaySound2D "/Game/Audio/SFX/DoorLocked.DoorLocked")
        (bind _asgame_mode_4 (Utilities|Casting|CastToGameMode (Game|GetGameMode)))
        (Default|WritetoArm _asgame_mode_4 "Repair Kit Required" false)))))

(fn ConstructionScript
  (|CallParentFunction))