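; Game mode for Derelict, a story game aboard a crippled ship, handling player spawn, transmissions and game end.
; On BeginPlay it spawns and possesses a VR or first-person pawn, and WriteToArm routes text to the VR arm or HUD to match.
; PlayDialog advances a counter selecting Chief Engineer Conrad's hardcoded transmissions, chained through PlayTimedDialog's sound, text and delay.
; EndGame shows a death message if oxygen is depleted, then fades out and quits.
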(event Custom|Write%20to%20Arm
  (params (TextToWrite :type String) (IsAlert :type Boolean))
  (if (Variables|Default|GetIsVR)
    (bind _asmotion_controller_pawn (Utilities|Casting|CastToMotionControllerPawn (Game|Player|GetPlayerPawn 0)))
    (Default|WritetoArm _asmotion_controller_pawn TextToWrite IsAlert)
    (else
      (bind _asfphud (Utilities|Casting|CastToFPHUD (HUD|GetHUD (Game|GetPlayerController 0))))
      (Default|WritetoHud _asfphud TextToWrite))))

(event Custom|End%20Game
  (if (<= (Variables|Default|GetPlayerOxygen) 0)
    (bind _asderelict_game_mode (Utilities|Casting|CastToDerelictGameMode (Game|GetGameMode)))
    (CallFunction|WritetoArm _asderelict_game_mode "You Died" false))
  (CameraFades|StartCameraFade :self (Game|GetPlayerCameraManager 0) :ToAlpha 1.0 :Duration 5.0 :bHoldWhenFinished true)
  (Utilities|FlowControl|Delay 7.0)
  (Game|QuitGame 0 "Quit" false))

(event Custom|PlayDialog
  (Variables|Default|SetDialogNum (+ (Variables|Default|GetDialogNum) 1))
  (if (== (Variables|Default|GetDialogNum) 1)
    (Utilities|FlowControl|Delay 5.0)
    (Utilities|PlayTimedDialog "INCOMING TRANSMISSION:" 5.0
      (:Return
        (Utilities|PlayTimedDialog "\"Hello?  This is Chief Engineer Conrad, who is this?\"" 6.0
          (:Return
            (Utilities|PlayTimedDialog "“Well, your voice transmission seems to be dead, but I'm guessing you don't exactly want to stick around here.  Our best hope is to send out an SOS from Comms.”" 1e+01
              (:Return
                (Utilities|PlayTimedDialog "“Unfortunately, the ship’s engine is down, and we’re running on aux power here.”" 7.0
                  (:Return
                    (Utilities|PlayTimedDialog "\"You fix enough power stations, you might be able to get main power back online.\"" 1e+01
                      (:Return
                        (Utilities|PlayTimedDialog "\"I don't have much juice left on this comm unit, but I'll contact you again once you get main power back on.\"" 3.0
                          (:Return
                            (Utilities|PlayTimedDialog "TRANMISSION ENDED" 1.0)))))))))))))
    (elif (== (Variables|Default|GetDialogNum) 2)
      (Utilities|PlayTimedDialog "INCOMING TRANSMISSION:" 5.0
        (:Return
          (Utilities|PlayTimedDialog "\"Okay, looks like we've got enough power to restore the core.  Just a warning, this will take all the power we've got.  Nothing else on the station will be powered.  So, make sure you're good to go!  We'll be out of here soon!  Don't worry about me, I'll meet you at the airlock once the SOS is out.\"" 3.0
            (:Return
              (Utilities|PlayTimedDialog "TRANMISSION ENDED" 1.0)))))
      (elif (== (Variables|Default|GetDialogNum) 3)
        (Utilities|PlayTimedDialog "INCOMING TRANSMISSION:" 5.0
          (:Return
            (Utilities|PlayTimedDialog "\"And, main power is back!  Now, if you can get that SOS out, we'll be home free!  The coms terminal should be back near engineering.  Good luck!\"" 3.0
              (:Return
                (Utilities|PlayTimedDialog "TRANMISSION ENDED" 1.0)))))
        (else
          (Utilities|PlayTimedDialog "INCOMING TRANSMISSION:" 5.0
            (:Return
              (Utilities|PlayTimedDialog "“Hey, there we go!  Our SOS signal is out!”" 5.0
                (:Return
                  (Utilities|PlayTimedDialog "“Well...your SOS signal.”" 5.0
                    (:Return
                      (Utilities|PlayTimedDialog "\"I'm afraid I haven't been entirely honest with you.  I...won't be meeting you at the airlock.\"" 7.0
                        (:Return
                          (Utilities|PlayTimedDialog "“I’ve heard you moving around the ship, so I’m guessing you’ve seen all the rooms but one.  I’m in the engine room.  And, umm...I don’t think I’ll be leaving it.”" 15.0
                            (:Return
                              (Utilities|PlayTimedDialog "“Our ship hit an asteroid field.  Punched right through the engine core.  I've done the math, the ship doesn't have the power to send the SOS and keep the engine leak contained.\" " 1e+01
                                (:Return
                                  (Utilities|PlayTimedDialog "“Which is why I disabled the door.   Permanently”" 5.0
                                    (:Return
                                      (Utilities|PlayTimedDialog "“So I won't be leaving here.  But...I'd like if it you could take my work with you.”" 7.0
                                        (:Return
                                          (Utilities|PlayTimedDialog "“The coms terminal should have uploaded the ship's databanks into your wrist computer.  Xenobiology.  Holographic tech.  Things I've put a lot of work into.”" 1e+01
                                            (:Return
                                              (Utilities|PlayTimedDialog "“A rescue drone should be here to pick you up shortly.  Probably at airlock 1.”" 7.0
                                                (:Return
                                                  (Utilities|PlayTimedDialog "\"And...it would mean a lot to me if you could get that information into the right hands.\"" 8.0
                                                    (:Return
                                                      (Utilities|PlayTimedDialog "\"Thank you.\"" 5.0
                                                        (:Return
                                                          (Utilities|PlayTimedDialog "TRANMISSION ENDED" 1.0))))))))))))))))))))))))))))))

(event EventBeginPlay
  (if (Variables|Default|GetIsVR)
    (bind _output_get (Variables|Default|SetDefaultPawnClass "/Game/VirtualReality/Blueprints/MotionControllerPawn.MotionControllerPawn_C"))
    (else
      (Variables|Default|SetDefaultPawnClass "/Game/Blueprints/FirstPersonCharacter.FirstPersonCharacter_C")))
  (bind _returnvalue (Game|SpawnActorfromClass _output_get (Transformation|GetActorTransform (Class|GameModeBase|FindPlayerStart (Game|GetPlayerController 0))) "Undefined" 0 0))
  (Pawn|Possess (Game|GetPlayerController 0) _returnvalue))

(fn ConstructionScript)